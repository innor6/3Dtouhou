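; Player controller for a level that tracks player health and a countdown and creates the Player_UI HUD on begin play.
; BeHited lowers HP with a sound, then either opens MainMenu when HP drops below zero or grants timed invulnerability that DeProtect clears.
; A looping one-second timer runs TimeDec, which opens the Staff level when time runs out.
; Escape returns to MainMenu.
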(event `self.ReceiveBeginPlay`
  (bind _returnvalue (`|CreateWidget` "/Game/level/Player_UI.Player_UI_C"))
  (bind _output_get (set `self.HUD Reference` _returnvalue))
  (`UserWidget.AddToViewport` _output_get 0)
  (bind _returnvalue_2 (`KismetSystemLibrary.K2_SetTimer` null "TimeDec" 1.0 true))
  (set `self.CntTimerHandle` _returnvalue_2))

(event `Key|Escape`
  (params (Key :type "Key Structure"))
  (:`Pressed`
    (`GameplayStatics.OpenLevel` "MainMenu")))

(fn `BeHited`
  (if (not (`self.Under Protected`))
    (bind _output_get (set `self.HP` (- (`self.HP`) 0.1)))
    (`GameplayStatics.PlaySound2D` "/Game/audio/pldead00.pldead00" 1.0 1.0 0.0 null null)
    (if (> 0.0 _output_get)
      (`GameplayStatics.OpenLevel` "MainMenu")
      (else
        (set `self.Under Protected` true)
        (bind _returnvalue (`KismetSystemLibrary.K2_SetTimer` null "DeProtect" 1.5)) ; 无敌时间
        (set `self.UPTimerHandle` _returnvalue)))))

(fn `DeProtect`
  (set `self.Under Protected` false)
  (`KismetSystemLibrary.K2_ClearAndInvalidateTimerHandle` (`self.UPTimerHandle`)))

(fn `TimeDec`
  (bind _output_get (set `self.Time` (- (`self.Time`) 1)))
  (if (<= _output_get 0)
    (`KismetSystemLibrary.K2_ClearAndInvalidateTimerHandle` (`self.CntTimerHandle`))
    (`GameplayStatics.OpenLevel` "Staff")))

(fn `UserConstructionScript`)